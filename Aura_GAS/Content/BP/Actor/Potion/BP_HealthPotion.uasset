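; BP_HealthPotion is a health potion pickup that uses the Gameplay Ability System.
; A sphere overlap passes the overlapping actor to ApplyEffectToTarget with its instant GameplayEffect class.
; A separate CreateEffectWidget event, skipped on authority, shows a centered pickup message with a red potion icon for the given player controller, then calls the widget's destroy event.
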(event OnComponentBeginOverlap(Sphere)
  (params (OverlappedComponent :type Primitive%20Component%20Object%20Reference) (OtherActor :type Actor%20Object%20Reference) (OtherComp :type Primitive%20Component%20Object%20Reference) (OtherBodyIndex :type Integer) (bFromSweep :type Boolean) (SweepResult :type Hit%20Result%20Structure%20%28by%20ref%29))
  (Class|AuraEffectActor|ApplyEffecttoTarget OtherActor (Variables|Default|GetInstanGameplayEffectClass)))

(event EventBeginPlay)

(event Collision|EventActorBeginOverlap
  (params (OtherActor :type Actor%20Object%20Reference)))

(event EventTick
  (params (DeltaSeconds :type Float%20%28single-precision%29)))

(event EventCreateEffectWidget
  (params (PlayerController :type Player%20Controller%20Object%20Reference))
  (if (not (Ability|HasAuthority))
    (bind _returnvalue (UserInterface|CreateWidget "/Game/BP/UI/Overlay/Subsystem/WBP_EffectMessage.WBP_EffectMessage_C" PlayerController))
    (Class|UserWidget|SetPositioninViewport _returnvalue (* (Viewport|GetViewportSize) 0.5) true)
    (Default|SetImageandText _returnvalue "Pick up a Health Potion" "/Game/Assets/UI/Pickups/T_Potion_Red.T_Potion_Red")
    (UserInterface|Viewport|AddtoViewport _returnvalue 0)
    (Default|CEDestoryWidget _returnvalue)))

(fn ConstructionScript)