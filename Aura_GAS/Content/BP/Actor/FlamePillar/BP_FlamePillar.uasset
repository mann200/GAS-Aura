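; BP_FlamePillar is a flame pillar actor whose FireLight flickers continuously from BeginPlay.
; It randomly plays one of two flame intensity timelines, then picks again when that finishes, creating an endless, varied loop.
; Each timeline update calls ScaleFlameIntensity, which multiplies the curve value by BaseIntensity to set the light's intensity.
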(event Custom|CE_StartTimeline_2
  (bind _flameintensity (Timeline|FlameIntensity_2 PlayFromStart)
    (:Update
      (CallFunction|ScaleFlameIntensity _flameintensity))
    (:Finished
      (CallFunction|CEChooseTimeline))))

(event Custom|CE_StartTimeline_1
  (bind _flameintensity (Timeline|FlameIntensity_1 PlayFromStart)
    (:Update
      (CallFunction|ScaleFlameIntensity _flameintensity))
    (:Finished
      (CallFunction|CEChooseTimeline))))

(event Custom|CE_ChooseTimeline
  (switch int (Math|Random|RandomIntegerinRange 0 1)
    (:0
      (CallFunction|CEStartTimeline1))
    (:1
      (CallFunction|CEStartTimeline2))))

(event EventBeginPlay
  (CallFunction|CEChooseTimeline))

(fn ConstructionScript)

(fn ScaleFlameIntensity
  (params (Intensity :type Float%20%28double-precision%29))
  (Rendering|Components|Light|SetIntensity (Variables|Default|GetFireLight) (* Intensity (Variables|Default|GetBaseIntensity))))