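; BP_EnemyBase is the base enemy character Blueprint, handling spawn scaling, attack-facing support and dissolve effects.
; On BeginPlay, a timeline drives the mesh's uniform relative scale.
; A facing event feeds a target location into Motion Warping as the "FacingTarget" warp target.
; Two dissolve events, one for the weapon, each run a timeline that animates the "Dissolve" parameter on a supplied dynamic material instance.
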(event EventBeginPlay
  (bind _dissolvetrack (Timeline|ScaleTrack Play)
    (:Update
      (Transformation|SetRelativeScale3D (Variables|Character|GetMesh) (Math|Vector|MakeVector _dissolvetrack _dissolvetrack _dissolvetrack)))))

(event Collision|EventActorBeginOverlap
  (params (OtherActor :type Actor%20Object%20Reference)))

(event EventTick
  (params (DeltaSeconds :type Float%20%28single-precision%29)))

(event EventStartDissolveTimeLine
  (params (DynamicMaterialInstance :type Material%20Instance%20Dynamic%20Object%20Reference))
  (bind _dissolvetrack (Timeline|DissolveTimeLine Play)
    (:Update
      (Rendering|Material|SetScalarParameterValue DynamicMaterialInstance "Dissolve" _dissolvetrack :!class /Script/Engine.MaterialInstanceDynamic))))

(event EventStartWeaponDissolveTimeLine
  (params (DynamicMaterialInstance :type Material%20Instance%20Dynamic%20Object%20Reference))
  (bind _weapondissolvetrack (Timeline|时间轴 Play)
    (:Update
      (Rendering|Material|SetScalarParameterValue DynamicMaterialInstance "Dissolve" _weapondissolvetrack :!class /Script/Engine.MaterialInstanceDynamic))))

(event EventUpdataFacingTarget
  (params (Target :type Vector%20%28by%20ref%29 :default "0, 0, 0"))
  (Class|MotionWarpingComponent|AddorUpdateWarpTargetfromLocation (Variables|Default|GetMotionWarping) "FacingTarget" Target))

(fn ConstructionScript)