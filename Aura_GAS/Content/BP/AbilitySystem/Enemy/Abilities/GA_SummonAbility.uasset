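; Enemy gameplay ability that plays a shaman summon montage and spawns random minions around the avatar.
; On activation it shuffles the spawn locations, then waits for the montage's attack event to start a delayed loop that spawns a ground effect and an AI-controlled minion at each point.
; Each spawn increments the avatar's minion count, and an OnDestroyed binding decrements it.
; The ability ends when the montage completes, blends out, or is interrupted or cancelled.
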(event Custom|OnDestroyed_事件
  (params (DestroyedActor :type Actor%20Object%20Reference))
  (Class|CombatInterface|IncremenetMinionCount(Message) (Ability|GetAvatarActorfromActorInfo) -1))

(event Ability|EventActivateAbility
  (bind _returnvalue (Class|AuraSummonAbility|GetSpawnLocation))
  (bind _output_get (Variables|Default|SetSpawnLocation _returnvalue))
  (Utilities|Array|Shuffle _output_get)
  (|PlayMontageandWaitProxy "None" "/Game/Assets/Enemies/Shaman/Animations/AM_Shamon_Summon.AM_Shamon_Summon" 1.0 "None" true 1.0 0.0 false
    (:then
      (Ability|Tasks|WaitGameplayEvent "(TagName=\"Montage.Attack.1\")" 0
        (:EventReceived
          (if (< (Variables|Default|GetSpawnLocationIndex) (Utilities|Array|Length (Variables|Default|GetSpawnLocation))) :!label _label
            (Niagara|SpawnSystematLocation "/Game/Assets/Effects/Combat/NS_GroundSummon.NS_GroundSummon" (Utilities|Array|Get(acopy) (Variables|Default|GetSpawnLocation) (Variables|Default|GetSpawnLocationIndex)))
            (bind _returnvalue_2 (Game|SpawnActorfromClass (Class|AuraSummonAbility|GetRandomMinionClass) (Math|Transform|MakeTransform (+ (Utilities|Array|Get(acopy) (Variables|Default|GetSpawnLocation) (Variables|Default|GetSpawnLocationIndex)) "0.000000,0.000000,70.000000") (Math|Rotator|FindLookatRotation (Transformation|GetActorLocation (Ability|GetAvatarActorfromActorInfo)) (+ (Utilities|Array|Get(acopy) (Variables|Default|GetSpawnLocation) (Variables|Default|GetSpawnLocationIndex)) "0.000000,0.000000,70.000000")) "1.000000,1.000000,1.000000") "Undefined" "MultiplyWithRoot" 0 0))
            (Game|AssignOnDestroyed _returnvalue_2 (delegate Custom|OnDestroyed_事件))
            (Pawn|SpawnDefaultController _returnvalue_2)
            (Class|CombatInterface|IncremenetMinionCount(Message) (Ability|GetAvatarActorfromActorInfo) 1)
            (Utilities|FlowControl|Delay 0.2)
            (Math|Integer|IncrementInt (Variables|Default|GetSpawnLocationIndex)
              (:%20%20
                (goto _label)))))))
    (:OnCompleted
      (Ability|EndAbility :!label _label_2))
    (:OnBlendOut
      (goto _label_2))
    (:OnInterrupted
      (goto _label_2))
    (:OnCancelled
      (goto _label_2))))

(event Ability|EventOnEndAbility
  (params (bWasCancelled :type Boolean)))