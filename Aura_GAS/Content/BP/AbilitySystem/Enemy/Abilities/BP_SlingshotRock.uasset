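; Projectile rock for an enemy slingshot ability that tumbles as it flies.
; BeginPlay picks random yaw, pitch and roll spin rates, which Tick scales by delta time to rotate the rock mesh locally.
; The Sphere collision switches to query-only after a short delay following spawn.
; The graph holds no overlap, movement or damage logic.
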(event EventBeginPlay
  (bind _returnvalue (Math|Random|RandomFloatinRange -3.6e+02 3.6e+02))
  (Variables|Default|SetYawRotationRale _returnvalue)
  (Variables|Default|SetPitchRotationRale _returnvalue)
  (Variables|Default|SetRollRotationRale _returnvalue)
  (Utilities|FlowControl|Delay 0.1)
  (Collision|SetCollisionEnabled (Variables|Default|GetSphere) "QueryOnly"))

(event Collision|EventActorBeginOverlap
  (params (OtherActor :type Actor%20Object%20Reference)))

(event EventTick
  (params (DeltaSeconds :type Float%20%28single-precision%29))
  (Transformation|AddLocalRotation (Variables|Default|GetRockMesh) (Math|Rotator|MakeRotator (* DeltaSeconds (Variables|Default|GetRollRotationRale)) (* DeltaSeconds (Variables|Default|GetPitchRotationRale)) (* DeltaSeconds (Variables|Default|GetYawRotationRale))) false false))

(fn ConstructionScript)