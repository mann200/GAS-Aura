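; GA_MeleeAttack is an enemy gameplay ability that performs a melee attack against the avatar's combat target.
; It turns to the target, plays a random tagged montage and waits for that montage's gameplay event.
; On the event, it damages non-friendly live players within a small radius of the tagged combat socket.
; Any hit fires one melee impact GameplayCue, and the ability ends without stopping the montage.
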(event Ability|EventActivateAbility
  (bind _returnvalue (Ability|GetAvatarActorfromActorInfo))
  (bind _returnvalue_2 (Ability|GetAvatarActorfromActorInfo))
  (Variables|Default|SetHasHitTarget false)
  (bind _returnvalue_3 (Class|EnemyInterface|GetCombatTarget(Message) _returnvalue_2))
  (Variables|Default|SetCombatTarget _returnvalue_3)
  (Class|CombatInterface|UpdataFacingTarget(Message) _returnvalue_2 (Transformation|GetActorLocation _returnvalue_3))
  (bind _returnvalue_4 (Class|CombatInterface|GetAttackMontages(Message) (Ability|GetAvatarActorfromActorInfo)))
  (Variables|Default|SetTaggedMontage (Class|AuraDamageGameplayAbility|GetRandomTaggedMontagefromArray _returnvalue_4))
  (|PlayMontageandWaitProxy "None" (.Montage (Utilities|Struct|BreakTaggedMontage (Variables|Default|GetTaggedMontage))) 1.0 "None" false 1.0 0.0 false
    (:then
      (Ability|Tasks|WaitGameplayEvent (.MontageTag (Utilities|Struct|BreakTaggedMontage (Variables|Default|GetTaggedMontage))) 0
        (:EventReceived
          (bind _returnvalue_5 (Class|CombatInterface|GetCombatSocketLocation(Message) _returnvalue (.SocketTag (Utilities|Struct|BreakTaggedMontage (Variables|Default|GetTaggedMontage)))))
          (bind _output_get (Variables|Default|SetCombatSocketLocation _returnvalue_5))
          (bind _outoverlappingactors (Class|AuraAbilitySystemLibrary|GetLivePlayersWithinRadius (Ability|GetAvatarActorfromActorInfo) (Utilities|Array|MakeArray _returnvalue) 45.0 _output_get))
          (for _array_element _outoverlappingactors
            (if (Class|AuraAbilitySystemLibrary|IsNotFriend (Ability|GetAvatarActorfromActorInfo) _array_element)
              (Class|AuraAbilitySystemLibrary|ApplyDamageEffect (Class|AuraDamageGameplayAbility|MakeDamageEffectParamsfromClassDefaults _array_element "0, 0, 0" false "0, 0, 0" false "0, 0, 0" false 0.0))
              (Variables|Default|SetHasHitTarget true)))
          (if (Variables|Default|GetHasHitTarget)
            (Class|GameplayAbility|ExecuteGameplayCuewithParams "(TagName=\"GameplayCue.MeleeImpact\")" (Ability|GameplayCue|MakeGameplayCueParameters :AggregatedSourceTags (GameplayTags|MakeGameplayTagContainerfromTag (.MontageTag (Utilities|Struct|BreakTaggedMontage (Variables|Default|GetTaggedMontage)))) :Location (Variables|Default|GetCombatSocketLocation) :EffectCauser (Ability|GetAvatarActorfromActorInfo) :SourceObject (Variables|Default|GetCombatTarget))))
          (Ability|EndAbility))))))