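; Gameplay ability that plays a hit reaction animation on the enemy that owns it.
; On activation it gets the montage from the avatar through CombatInterface, plays it with a wait task, and ends when the montage completes, is interrupted or is cancelled.
; Disconnected leftover nodes hold earlier approaches that froze walk speed, set the HitReacting blackboard key or applied GE_HitReact with a granted tag; none of them run.
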(event Ability|EventOnEndAbility
  (params (bWasCancelled :type Boolean)))

(event Ability|EventActivateAbility
  (bind _ascombat_interface (Utilities|Casting|CastToCombatInterface (Ability|GetAvatarActorfromActorInfo)))
  (bind _returnvalue (Class|CombatInterface|GetHitReactMontage _ascombat_interface))
  (|PlayMontageandWaitProxy "None" _returnvalue 1.0 "None" true 1.0 0.0 false
    (:OnCompleted
      _)
    (:OnInterrupted
      _)
    (:OnCancelled
      _))
  (Ability|EndAbility))