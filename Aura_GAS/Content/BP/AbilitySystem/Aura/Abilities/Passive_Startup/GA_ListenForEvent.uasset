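; GA_ListenForEvent is a passive startup gameplay ability that turns Attributes gameplay events into effects on its owner.
; On activation it waits for events under the Attributes tag, child tags included, then builds a spec from EventBasedEffectClass.
; It sets every EventTags entry as a SetByCaller magnitude, using the event magnitude for the exact match and zero for the rest, then applies the spec to the owner.
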(event Ability|EventActivateAbility
  (bind _payload (Ability|Tasks|WaitGameplayEvent "(TagName=\"Attributes\")" 0 false false)
    (:EventReceived
      (Variables|Default|SetEvent%20Tag (.EventTag (Utilities|Struct|BreakGameplayEventData _payload)))
      (Variables|Default|SetEvent%20Magnitude (.EventMagnitude (Utilities|Struct|BreakGameplayEventData _payload)))
      (Variables|Default|SetSpecHandle (Ability|MakeOutgoingGameplayEffectSpec (Variables|Default|GetEventBasedEffectClass)))
      (for _array_element (Variables|Default|GetEventTags)
        (if (GameplayTags|MatchesTag _array_element (Variables|Default|GetEvent%20Tag) true)
          (Ability|GameplayEffect|AssignTagSetbyCallerMagnitude (Variables|Default|GetSpecHandle) (Variables|Default|GetEvent%20Tag) (Variables|Default|GetEvent%20Magnitude))
          (else
            (Ability|GameplayEffect|AssignTagSetbyCallerMagnitude (Variables|Default|GetSpecHandle) _array_element 0.0))))
      (Ability|ApplyGameplayEffectSpecToOwner (Variables|Default|GetSpecHandle)))))