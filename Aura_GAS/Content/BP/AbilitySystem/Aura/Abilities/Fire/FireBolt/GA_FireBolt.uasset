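; GA_FireBolt is a gameplay ability that casts fire bolt projectiles at the target under the mouse.
; It commits, takes the hit location and actor from mouse target data, and turns the caster toward that point through CombatInterface.
; A cast montage plays, and its FireBolt event tag triggers SpawnProjectiles from the weapon socket with a pitch override and the hit actor as homing target.
; The ability ends when the montage completes, blends out, or is interrupted or cancelled.
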(event Ability|EventActivateAbility
  (Ability|CommitAbility)
  (bind _data (|TargetDataUnderMouse)
    (:ValidData
      (bind _output_get (Variables|Default|SetProjectile%20Target%20Location (.Location (Collision|BreakHitResult (Ability|TargetData|GetHitResultfromTargetData _data)))))
      (Variables|Default|SetMouse%20Hit%20Actor (.HitActor (Collision|BreakHitResult (Ability|TargetData|GetHitResultfromTargetData _data))))
      (bind _ascombat_interface (Utilities|Casting|CastToCombatInterface (Ability|GetAvatarActorfromActorInfo)))
      (Class|CombatInterface|UpdataFacingTarget _ascombat_interface _output_get)
      (|PlayMontageandWaitProxy "None" "/Game/Assets/Characters/Aura/Animations/Abilities/AM_Cast_FireBolt.AM_Cast_FireBolt" 1.0 "None" false 1.0 0.0 false
        (:then
          (Ability|Tasks|WaitGameplayEvent "(TagName=\"Event.Montage.FireBolt\")" 0
            (:EventReceived
              (Class|AuraFireBolt|SpawnProjectiles (Variables|Default|GetProjectile%20Target%20Location) (GameplayTags|MakeLiteralGameplayTag "(TagName=\"CombatSocket.Weapon\")") true 45.0 (Variables|Default|GetMouse%20Hit%20Actor)))))
        (:OnCompleted
          (Ability|EndAbility :!label _label))
        (:OnBlendOut
          (goto _label))
        (:OnInterrupted
          (goto _label))
        (:OnCancelled
          (goto _label))))))

(event Ability|EventOnEndAbility
  (params (bWasCancelled :type Boolean)))